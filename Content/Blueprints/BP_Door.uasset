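; BP_Door is a locked door that the player opens by spending a key.
; When BP_ThirdPersonCharacter overlaps the actor, it prints a knocking message and checks the character's TotalKeys.
; With a key available, it decrements the count and destroys the SMBldDoor01 and OverlapBox components, removing the door permanently rather than animating it.
; Without one, it prints a prompt to find a key.
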(event EventBeginPlay)

(event Collision|EventActorBeginOverlap
  (params (OtherActor :type Actor%20Object%20Reference))
  (bind _asbp_third_person_character (Utilities|Casting|CastToBP_ThirdPersonCharacter OtherActor))
  (Development|PrintText "The player is knocking")
  (if (> (Variables|/Game/ThirdPerson/Blueprints/BP_ThirdPersonCharacter.BP_ThirdPersonCharacter_C|GetTotalKeys _asbp_third_person_character) 0) ; If they have a key,\nOpen a door\nElse,\nlaugh at them
    (Math|Integer|DecrementInt (Variables|/Game/ThirdPerson/Blueprints/BP_ThirdPersonCharacter.BP_ThirdPersonCharacter_C|GetTotalKeys _asbp_third_person_character)
      (:%20%20
        (Components|DestroyComponent (Variables|Default|GetSM_Bld_Door_01))
        (Components|DestroyComponent (Variables|Default|GetOverlapBox))))
    (else
      (Development|PrintText "Find a key!"))))

(event EventTick
  (params (DeltaSeconds :type Float%20%28single-precision%29)))

(fn ConstructionScript)