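; BP_DialogueManager shows dialogue lines on screen through a W_Dialogue widget created at BeginPlay.
; DisplayNextLine prints a random Dialogue entry and sets a separately randomized one on the widget, so the two can differ.
; The widget leaves the viewport after a delay, while Index increments immediately.
; Index only counts displays, resetting at the array's end if ShouldRepeatText is set; otherwise display stops.
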(event Custom|DisplayNextLine
  (bind _dialogue (Variables|Default|GetDialogue))
  (bind _dialoguewidget (Variables|Default|GetDialogueWidget))
  (bind _outitem (Utilities|Array|Random _dialogue))
  (if (>= (Variables|Default|GetIndex) (Utilities|Array|Length (Variables|Default|GetDialogue)))
    (if (Variables|Default|GetShouldRepeatText)
      (Variables|Default|SetIndex 0)
      (Development|PrintText _outitem true true "(R=0.482144,G=1.000000,B=0.477435,A=1.000000)" 5.0 :!label _label)
      (Rendering|Components|TextRender|SetText (Variables|/Game/Widgets/W_Dialogue.W_Dialogue_C|GetTextBlock_0 _dialoguewidget) _outitem)
      (Utilities|FlowControl|Sequence
        (:then_0
          (UserInterface|Viewport|AddtoViewport _dialoguewidget 0)
          (Utilities|FlowControl|Delay 5.0)
          (Widget|RemovefromParent _dialoguewidget))
        (:then_1
          (Math|Integer|IncrementInt (Variables|Default|GetIndex)))))
    (else
      (goto _label))))

(event EventBeginPlay
  (bind _returnvalue (UserInterface|CreateWidget "/Game/Widgets/W_Dialogue.W_Dialogue_C"))
  (Variables|Default|SetDialogueWidget _returnvalue))

(fn ConstructionScript)