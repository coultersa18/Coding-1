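; BP_Fertilizer is a cone-mesh pickup that gives the third-person character a random amount of fertilizer on overlap.
; It passes the amount to the character's GetFertilizerCount, then hides its mesh and disables its collision.
; After a short delay, it spawns a replacement of its own class at a random point in a hardcoded rectangle at fixed height, then destroys itself.
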(event Custom|Respawn%20Fertilizer
  (Game|SpawnActorfromClass "BP_Fertilizer_C" (Math|Transform|MakeTransform (Math|Vector|MakeVector (Math|Random|RandomFloatinRange -135.0 -9.2e+02) (Math|Random|RandomFloatinRange 2.3e+02 9e+02) 7e+01) "0, 0, 0" "1.000000,1.000000,1.000000") "Undefined" "MultiplyWithRoot" 0 0)
  (Development|PrintText "Fertilizer respawned!"))

(event EventBeginPlay)

(event Collision|EventActorBeginOverlap
  (params (OtherActor :type Actor%20Object%20Reference))
  (bind _asbp_third_person_character (Utilities|Casting|CastToBP_ThirdPersonCharacter OtherActor))
  (Default|GetFertilizerCount _asbp_third_person_character (Math|Random|RandomIntegerinRange 2 6))
  (Development|SetHiddeninGame (Variables|Default|GetSM_PolygonPrototype_Prop_Cone_01) true false)
  (Collision|SetActorEnableCollision false)
  (Utilities|FlowControl|Delay 4.0)
  (CallFunction|RespawnFertilizer)
  (Actor|DestroyActor))

(event EventTick
  (params (DeltaSeconds :type Float%20%28single-precision%29)))

(fn ConstructionScript)