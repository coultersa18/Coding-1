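; BP_LoopsandLists is an actor Blueprint that demonstrates loop and array techniques, mainly by randomly rotating BP_Tree actors.
; BeginPlay starts SimpleLoop, a Delay-driven endless cycle that triggers LoopArrayOverTime to turn trees one at a time using an index and short delays.
; It also runs WhileLoopFunction, a counter countdown printing timestamped messages in cycling colors.
; ChangeTreesForEach rotates all trees at once but is uncalled here, and a Shuffle node is unwired.
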(event Custom|SimpleLoop
  (Development|PrintText "Inside Simple Loop waiting 3 seconds" :!label _label)
  (CallFunction|LoopArrayOverTime)
  (Utilities|FlowControl|Delay 3.0)
  (goto _label))

(event Custom|WhileLoopFunction
  (bind _colors (Variables|Default|GetColors))
  (while (> (Variables|Default|GetWhileCounter) 0)
    (Development|PrintText (Utilities|Text|FormatText "This is loop {count} Ran after {seconds} seconds." (Variables|Default|GetWhileCounter) (Utilities|Text|ToText(Float) (Utilities|Time|GetRealTimeSeconds) "HalfToEven" false true 1 324 3)) true true (Utilities|Array|Get(acopy) _colors (Math|Integer|%(Integer) (Variables|Default|GetWhileCounter) (Utilities|Array|Length _colors))) 2e+01)
    (Math|Integer|DecrementInt (Variables|Default|GetWhileCounter))))

(event Custom|ChangeTreesForEach
  (bind _outactors (Actor|GetAllActorsOfClass "/Game/Blueprints/BP_Tree.BP_Tree_C"))
  (for _array_element _outactors
    (Transformation|SetActorRelativeRotation _array_element (Math|Rotator|MakeRotator 0.0 0.0 (Math|Random|RandomFloatinRange 0.0 3.6e+02))))
  (Development|PrintText "Trees have been rotated"))

(event Custom|LoopArrayOverTime
  (bind _outactors (Actor|GetAllActorsOfClass "/Game/Blueprints/BP_Tree.BP_Tree_C"))
  (if (< (Variables|Default|GetOvertimeIndex) (Utilities|Array|Length _outactors)) :!label _label
    (Transformation|SetActorRelativeRotation (Utilities|Array|Get(acopy) _outactors (Variables|Default|GetOvertimeIndex)) (Math|Rotator|MakeRotator 0.0 0.0 (Math|Random|RandomFloatinRange 0.0 3.6e+02)))
    (Math|Integer|IncrementInt (Variables|Default|GetOvertimeIndex)
      (:%20%20
        (Utilities|FlowControl|Delay 0.2)
        (goto _label)))
    (else
      (Variables|Default|SetOvertimeIndex 0))))

(event EventBeginPlay
  (Development|PrintText "Loops and Lists is starting")
  (CallFunction|SimpleLoop)
  (CallFunction|WhileLoopFunction))

(event Collision|EventActorBeginOverlap
  (params (OtherActor :type Actor%20Object%20Reference)))

(event EventTick
  (params (DeltaSeconds :type Float%20%28single-precision%29)))

(fn ConstructionScript)