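; BP_Cannon is an actor that fires a cannonball automatically every second from the start of play.
; BeginPlay runs an endless delay loop that calls the FireCannon event.
; FireCannon prints a message, spawns a BP_CannonBall at the SpawnPoint transform and pushes its Cube along that component's forward vector, using a mass-independent AddForce.
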(event Custom|FireCannon
  (Development|PrintText "Cannon is firing" true true "(R=0.000000,G=0.660000,B=1.000000,A=1.000000)" 1.0)
  (bind _returnvalue (Game|SpawnActorfromClass "/Game/Blueprints/BP_CannonBall.BP_CannonBall_C" (Transformation|GetWorldTransform (Variables|Default|GetSpawnPoint)) "Undefined" "MultiplyWithRoot" 0 0))
  (Physics|AddForce (Variables|/Game/Blueprints/BP_CannonBall.BP_CannonBall_C|GetCube _returnvalue) (* (Math|Vector|GetForwardVector (Variables|Default|GetSpawnPoint)) 1e+05) "None" true))

(event EventBeginPlay
  (Utilities|FlowControl|Delay 1.0 :!label _label)
  (CallFunction|FireCannon)
  (goto _label))

(fn ConstructionScript)