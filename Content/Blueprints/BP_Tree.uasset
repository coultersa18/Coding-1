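; BP_Tree is a tree actor that the player fertilizes with F while overlapping its FertilizerCheck, spending one of the character's fertilizer.
; A DoN with a random limit loops through delayed Grow calls, each randomly enlarging SMTree and advancing BP_DialogueManager's dialogue.
; A zero counter check ends the loop, switching collision from FertilizerCheck to the tree mesh.
; Actor overlap adds a text render component, and the HasBeenFertilized flag must be true to allow fertilizing.
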(event Custom|Grow
  (bind _sm_tree (Variables|Default|GetSM_Tree))
  (Transformation|SetRelativeScale3D _sm_tree (+ (Variables|/Script/Engine.SceneComponent|GetRelativeScale3D _sm_tree) (Math|Random|RandomFloatinRange 0.2 0.6))))

(event EventBeginPlay
  (Input|EnableInput (Game|GetPlayerController 0))
  (bind _returnvalue (Actor|GetActorOfClass "/Game/Blueprints/BP_DialogueManager.BP_DialogueManager_C"))
  (Variables|Default|SetDialoguemanager _returnvalue))

(event Collision|EventActorBeginOverlap
  (params (OtherActor :type Actor%20Object%20Reference))
  (AddComponent|AddTextRenderComponent false))

(event Input|KeyboardEvents|F
  (params (Key :type Key%20Structure :default "None"))
  (:Pressed
    (if (Variables|Default|GetHasBeenFertilized)
      (if (Collision|IsOverlappingActor (Variables|Default|GetFertilizerCheck) (stale Collision|EventActorBeginOverlap OtherActor) :!class /Script/Engine.PrimitiveComponent)
        (bind _asbp_third_person_character (Utilities|Casting|CastToBP_ThirdPersonCharacter (stale Collision|EventActorBeginOverlap OtherActor)))
        (bind _returnvalue (Actor|GetActorOfClass "/Game/ThirdPerson/Blueprints/BP_ThirdPersonCharacter.BP_ThirdPersonCharacter_C"))
        (if (> (Variables|/Game/ThirdPerson/Blueprints/BP_ThirdPersonCharacter.BP_ThirdPersonCharacter_C|GetTotalFertilizerCount _returnvalue) 0)
          (Variables|Default|SetHasBeenFertilized false)
          (Default|GetFertilizerCount _asbp_third_person_character -1)
          (bind _counter (Utilities|FlowControl|DoN (Math|Random|RandomIntegerinRange 1 5) :!label _label)
            (:Exit
              (Utilities|FlowControl|Delay (Math|Random|RandomFloatinRange 3.0 5.0))
              (CallFunction|Grow)
              (Utilities|Casting|CastToBP_ThirdPersonCharacter (stale Collision|EventActorBeginOverlap OtherActor))
              (Default|DisplayNextLine (Variables|Default|GetDialoguemanager))
              (if (== _counter 0)
                (Collision|SetCollisionEnabled (Variables|Default|GetSM_Tree) "QueryAndPhysics")
                (Collision|SetCollisionEnabled (Variables|Default|GetFertilizerCheck) "NoCollision")
                (Development|PrintText "Collision Enabled!")
                (else
                  (goto _label)))))
          (else
            (Development|PrintText "You have no more fertilizer!")))))))

(fn ConstructionScript)